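; BP_StageCamera is a player-controllable stage camera on a spring arm, with yaw, pitch, zoom and reset.
; It registers IMC_Camera on BeginPlay; its Enhanced Input actions set clamped target angles and a distance bounded relative to BaseDist.
; Tick eases the arm toward those targets.
; Shake sets an amplitude that Tick applies as random camera offsets and decays to zero.
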(event `self.ReceiveBeginPlay`
  (bind _returnvalue (`GameplayStatics.GetPlayerController` 0))
  (set `self.TargetDist` (`self.BaseDist`))
  (`self.EnableInput` _returnvalue)
  (message `EnhancedInputSubsystemInterface.AddMappingContext` (`SubsystemBlueprintLibrary.GetLocalPlayerSubSystemFromPlayerController` _returnvalue "/Script/EnhancedInput.EnhancedInputLocalPlayerSubsystem") "/Game/ShrinkRooms/Player/IMC_Camera.IMC_Camera" 0 (struct)))

(event `self.ReceiveTick`
  (params (DeltaSeconds :type "Float (single-precision)"))
  (`SceneComponent.K2_SetRelativeRotation` (`self.Arm`) (`KismetMathLibrary.RInterpTo` (`SceneComponent.K2_GetComponentRotation` (`self.Arm`)) (`KismetMathLibrary.MakeRotator` 0.0 (`self.TargetPitch`) (`self.TargetYaw`)) DeltaSeconds 8.0) false false)
  (set `SpringArmComponent.TargetArmLength` (`KismetMathLibrary.FInterpTo` (`SpringArmComponent.TargetArmLength` (`self.Arm`)) (`self.TargetDist`) DeltaSeconds 8.0) (`self.Arm`))
  (`SceneComponent.K2_SetRelativeLocation` (`self.Cam`) (* (`KismetMathLibrary.RandomUnitVector`) (`self.ShakeAmp`)) false false)
  (set `self.ShakeAmp` (`KismetMathLibrary.FInterpTo` (`self.ShakeAmp`) 0.0 DeltaSeconds 7.0)))

(event `EnhancedInput|/Game/ShrinkRooms/Player/IA_CamYaw`
  (params (ActionValue :type "Float (double-precision)") (ElapsedSeconds :type "Float (double-precision)") (TriggeredSeconds :type "Float (double-precision)") (InputAction :type "InputAction Object Reference" :default "/Game/ShrinkRooms/Player/IA_CamYaw.IA_CamYaw"))
  (:`Triggered`
    (set `self.TargetYaw` (`KismetMathLibrary.FClamp` (+ (`self.TargetYaw`) (* (* ActionValue 90.0) (`GameplayStatics.GetWorldDeltaSeconds`))) -70.0 70.0))))

(event `EnhancedInput|/Game/ShrinkRooms/Player/IA_CamPitch`
  (params (ActionValue :type "Float (double-precision)") (ElapsedSeconds :type "Float (double-precision)") (TriggeredSeconds :type "Float (double-precision)") (InputAction :type "InputAction Object Reference" :default "/Game/ShrinkRooms/Player/IA_CamPitch.IA_CamPitch"))
  (:`Triggered`
    (set `self.TargetPitch` (`KismetMathLibrary.FClamp` (+ (`self.TargetPitch`) (* (* ActionValue 45.0) (`GameplayStatics.GetWorldDeltaSeconds`))) -88.0 -30.0))))

(event `EnhancedInput|/Game/ShrinkRooms/Player/IA_CamZoom`
  (params (ActionValue :type "Float (double-precision)") (ElapsedSeconds :type "Float (double-precision)") (TriggeredSeconds :type "Float (double-precision)") (InputAction :type "InputAction Object Reference" :default "/Game/ShrinkRooms/Player/IA_CamZoom.IA_CamZoom"))
  (:`Triggered`
    (set `self.TargetDist` (`KismetMathLibrary.FClamp` (- (`self.TargetDist`) (* ActionValue 80.0)) (* (`self.BaseDist`) 0.5) (* (`self.BaseDist`) 1.5)))))

(event `EnhancedInput|/Game/ShrinkRooms/Player/IA_CamReset`
  (params (ActionValue :type Boolean) (ElapsedSeconds :type "Float (double-precision)") (TriggeredSeconds :type "Float (double-precision)") (InputAction :type "InputAction Object Reference" :default "/Game/ShrinkRooms/Player/IA_CamReset.IA_CamReset"))
  (:`Started`
    (set `self.TargetPitch` -60.0)
    (set `self.TargetYaw` 0.0)
    (set `self.TargetDist` (`self.BaseDist`))))

(fn `Shake`
  (params (Amount :type "Float (single-precision)"))
  (set `self.ShakeAmp` Amount))

(fn `UserConstructionScript`)