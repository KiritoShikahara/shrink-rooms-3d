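; Base actor for objects placed on a grid in ShrinkRooms, carrying cell coordinates and blocking and pushable flags.
; SnapToGrid turns the cell into a target location with X and Y swapped, which Tick eases toward after BeginPlay starts the actor at world origin.
; Tick's squash-and-stretch scaling has a constant zero input, leaving the mesh at base scale.
; RemoveFromGrid moves coordinates off-grid, clears both flags and hides the actor.
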(event `self.ReceiveBeginPlay`
  (`self.SnapToGrid`)
  (`self.K2_SetActorLocation` (0.0 0.0 0.0))
  (`PrimitiveComponent.SetMaterial` (`self.Mesh`) 0 (`self.BodyMaterial`))
  (`SceneComponent.SetRelativeScale3D` (`self.Mesh`) (`self.MeshScale`)))

(event `self.ReceiveTick`
  (params (DeltaSeconds :type "Float (single-precision)"))
  (bind _returnvalue (`KismetMathLibrary.FClamp` 0.0 0.0 1.0))
  (`self.K2_SetActorLocation` (`KismetMathLibrary.VInterpTo` (`self.K2_GetActorLocation`) (`self.TargetLocation`) DeltaSeconds (`self.InterpSpeed`)))
  (`SceneComponent.SetRelativeScale3D` (`self.Mesh`) (`KismetMathLibrary.MakeVector` (* (.x (`self.MeshScale`)) (+ 1.0 (* _returnvalue 0.12))) (* (.y (`self.MeshScale`)) (+ 1.0 (* _returnvalue 0.12))) (* (.z (`self.MeshScale`)) (+ 1.0 (* _returnvalue -0.18))))))

(fn `RemoveFromGrid`
  (set `self.GridX` -999)
  (set `self.GridY` -999)
  (set `self.BlocksMovement` false)
  (set `self.Pushable` false)
  (`self.SetActorHiddenInGame` true))

(fn `SnapToGrid`
  (set `self.TargetLocation` (`KismetMathLibrary.MakeVector` (* (`self.GridY`) (`self.CellSize`)) (* (`self.GridX`) (`self.CellSize`)) (`self.MeshZ`))))

(fn `UserConstructionScript`)