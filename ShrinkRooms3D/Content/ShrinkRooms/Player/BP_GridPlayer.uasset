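; BP_GridPlayer is the player-controlled actor in a turn-based grid game, registering with BP_GridManager on BeginPlay.
; Enhanced Input move presses become integer grid steps, while retry restarts the stage through BP_GameInstance.
; Step asks the manager to validate moves while its game state is zero, advancing the turn on success with a pitch-randomized sound.
; Blocked moves play a bump sound and nudge the actor toward the attempted direction.
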(event `self.ReceiveBeginPlay`
  (bind _returnvalue (`GameplayStatics.GetPlayerController` 0))
  (`parent.ReceiveBeginPlay`)
  (bind _returnvalue_2 (`GameplayStatics.GetActorOfClass` "/Game/ShrinkRooms/Core/BP_GridManager.BP_GridManager_C"))
  (set `self.Manager` _returnvalue_2)
  (`/Game/ShrinkRooms/Core/BP_GridManager.RegisterPlayer` (`self.Manager`) self)
  (`self.EnableInput` _returnvalue)
  (message `EnhancedInputSubsystemInterface.AddMappingContext` (`SubsystemBlueprintLibrary.GetLocalPlayerSubSystemFromPlayerController` _returnvalue "/Script/EnhancedInput.EnhancedInputLocalPlayerSubsystem") "/Game/ShrinkRooms/Player/IMC_Default.IMC_Default" 0 (struct)))

(event `EnhancedInput|/Game/ShrinkRooms/Player/IA_Move`
  (params (ActionValue :type "Vector2D Structure") (ElapsedSeconds :type "Float (double-precision)") (TriggeredSeconds :type "Float (double-precision)") (InputAction :type "InputAction Object Reference" :default "/Game/ShrinkRooms/Player/IA_Move.IA_Move"))
  (bind (_x _y) (`KismetMathLibrary.BreakVector2D` ActionValue))
  (:`Started`
    (`self.Step` (`KismetMathLibrary.Round` _x) (`KismetMathLibrary.Round` _y))))

(event `EnhancedInput|/Game/ShrinkRooms/Player/IA_Retry`
  (params (ActionValue :type Boolean) (ElapsedSeconds :type "Float (double-precision)") (TriggeredSeconds :type "Float (double-precision)") (InputAction :type "InputAction Object Reference" :default "/Game/ShrinkRooms/Player/IA_Retry.IA_Retry"))
  (:`Started`
    (bind _asbp_game_instance (cast `/Game/ShrinkRooms/Core/BP_GameInstance` (`GameplayStatics.GetGameInstance`)))
    (`/Game/ShrinkRooms/Core/BP_GameInstance.RestartStage` _asbp_game_instance)))

(fn `Step`
  (params (DX :type Integer) (DY :type Integer))
  (if (== (`/Game/ShrinkRooms/Core/BP_GridManager.GameState` (`self.Manager`)) 0)
    (bind _success (`/Game/ShrinkRooms/Core/BP_GridManager.TryMove` (`self.Manager`) self DX DY))
    (if _success
      (`GameplayStatics.PlaySound2D` "/Game/ShrinkRooms/Art/Audio/sfx_move1.sfx_move1" 1.0 (`KismetMathLibrary.RandomFloatInRange` 0.9 1.15) 0.0 null null)
      (`/Game/ShrinkRooms/Core/BP_GridManager.AdvanceTurn` (`self.Manager`))
      (else
        (`GameplayStatics.PlaySound2D` "/Game/ShrinkRooms/Art/Audio/sfx_bump.sfx_bump" 1.0 1.0 0.0 null null)
        (`self.K2_SetActorLocation` (+ (`self.K2_GetActorLocation`) (`KismetMathLibrary.MakeVector` (* (`KismetMathLibrary.Conv_IntToDouble` DY) 8.0) (* (`KismetMathLibrary.Conv_IntToDouble` DX) 8.0))))))))

(fn `UserConstructionScript`
  (`parent.UserConstructionScript`))